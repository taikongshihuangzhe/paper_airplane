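; Base enemy Blueprint that handles health, damage and death for enemies in a game run by plane_gameMode.
; On BeginPlay it adds itself to the game mode's enemy count and sets Health to MaxHealth.
; GotHit subtracts damage when DamageEnabled is set and calls Death at zero health or below.
; SetDeathTimer schedules the same Death event, which destroys the actor without decrementing the count here.
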(event Custom|Got%20Hit
  (params (Damage :type Float%20%28single-precision%29))
  ;[1 0 0] Damage
  (if (Variables|Default|GetDamageEnabled)
    (CallFunction|CalculateDamage Damage)
    (bind _dead (CallFunction|GetIsDead))
    (if _dead
      (CallFunction|Death))))

(event Custom|Set%20Death%20Timer
  (params (time :type Float%20%28single-precision%29))
  ;[0 0.4584 1] Life Time
  (Utilities|Time|SetTimerbyEvent (delegate Custom|Death) time))

(event Custom|Death
  (Actor|DestroyActor))

(event EventBeginPlay
  ;[1 1 1] Initianization
  (bind _asplane_game_mode (Utilities|Casting|CastToplane_gameMode (Game|GetGameMode)))
  (bind _output_get (Variables|Default|SetBP_GameMode _asplane_game_mode))
  (Default|UpdateEnemyCount _output_get 1)
  (Variables|Default|SetHealth (Variables|Default|GetMaxHealth)))

(fn ConstructionScript)

(fn CalculateDamage
  (params (input_damage :type Float%20%28single-precision%29))
  (Variables|Default|SetHealth (- (Variables|Default|GetHealth) input_damage)))

(fn GetIsDead
  (return (<= (Variables|Default|GetHealth) 0.0)))