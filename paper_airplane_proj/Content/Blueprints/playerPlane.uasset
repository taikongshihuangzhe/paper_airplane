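; Player plane that follows the player's finger on a horizontal plane at the first PlayerStart's height.
; Touch press and move call TouchToWorld, which intersects the deprojected camera ray with that plane to set the target location.
; Tick eases toward the target with a swept move, setting yaw from Y velocity scaled by the Yaw variable.
; LocationSpaceSwitch, a rougher scaled-direction conversion, is not called in this graph.
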(event EventTick
  (params (DeltaSeconds :type Float%20%28single-precision%29))
  (bind _returnvalue (Transformation|GetActorLocation))
  ;[1 1 1] movement
  (Variables|Default|SetdeltaSec DeltaSeconds)
  (Transformation|SetActorLocationAndRotation (Math|Vector|MakeVector (.x (Class|KismetMathLibrary|Vector2DInterpto (Math|Vector2D|MakeVector2D (.x _returnvalue) (.y _returnvalue)) (Variables|Default|GettargetLocation) (Variables|Default|GetdeltaSec) 4.0)) (.y (Class|KismetMathLibrary|Vector2DInterpto (Math|Vector2D|MakeVector2D (.x _returnvalue) (.y _returnvalue)) (Variables|Default|GettargetLocation) (Variables|Default|GetdeltaSec) 4.0)) (.z (stale Input|TouchEvents|InputTouch _3doutput))) (Math|Rotator|MakeRotator 0.0 0.0 (* (/ (- (.y (Class|KismetMathLibrary|Vector2DInterpto (Math|Vector2D|MakeVector2D (.x _returnvalue) (.y _returnvalue)) (Variables|Default|GettargetLocation) (Variables|Default|GetdeltaSec) 4.0)) (.y _returnvalue)) (Variables|Default|GetdeltaSec)) (Variables|Default|Getyaw))) true))

(event Input|TouchEvents|InputTouch
  (params (Location :type Vector) (FingerIndex :type ETouchIndex%20Enum))
  ;[1 1 1] movement
  (:Pressed
    (bind _3doutput (CallFunction|TouchtoWorld Location :!label _label))
    (Variables|Default|SettargetLocation (Math|Vector2D|MakeVector2D (.x _3doutput) (.y _3doutput))))
  (:Moved
    (goto _label)))

(fn ConstructionScript)

(fn LocationSpaceSwitch
  (params (touchInput :type Vector))
  (bind _returnvalue (Game|GetPlayerController 0))
  (bind (_worldposition _worlddirection _returnvalue_2) (Class|GameplayStatics|DeprojectScreentoWorld _returnvalue (Math|Vector2D|MakeVector2D (.x touchInput) (.y touchInput))))
  (bind _outactors (Actor|GetAllActorsOfClass "/Script/Engine.PlayerStart"))
  (if _returnvalue_2
    (bind _output_get (Variables|Default|Setalpha (/ (.z (Camera|GetCameraLocation (Game|GetPlayerCameraManager 0))) (.z (Transformation|GetActorLocation (Utilities|Array|Get(acopy) _outactors))))))
    (return (Math|Vector|MakeVector (.x (+ (Math|Vector2D|MakeVector2D (.x (Transformation|GetActorLocation (Utilities|Array|Get(acopy) _outactors))) (.y (Transformation|GetActorLocation (Utilities|Array|Get(acopy) _outactors)))) (* (Math|Vector2D|MakeVector2D (.x _worlddirection) (.y _worlddirection)) (* 5.0 _output_get)))) (.y (+ (Math|Vector2D|MakeVector2D (.x (Transformation|GetActorLocation (Utilities|Array|Get(acopy) _outactors))) (.y (Transformation|GetActorLocation (Utilities|Array|Get(acopy) _outactors)))) (* (Math|Vector2D|MakeVector2D (.x _worlddirection) (.y _worlddirection)) (* 5.0 _output_get)))) (.z (Transformation|GetActorLocation (Utilities|Array|Get(acopy) _outactors)))))))

(fn TouchtoWorld
  (params (touchInput :type Vector))
  (bind _returnvalue (Game|GetPlayerController 0))
  (bind _returnvalue_2 (Game|GetPlayerCameraManager 0))
  (bind _returnvalue_3 (Camera|GetCameraLocation _returnvalue_2))
  (bind (_worldposition _worlddirection _returnvalue_4) (Class|GameplayStatics|DeprojectScreentoWorld _returnvalue (Math|Vector2D|MakeVector2D (.x touchInput) (.y touchInput))))
  (bind _outactors (Actor|GetAllActorsOfClass "/Script/Engine.PlayerStart"))
  (if _returnvalue_4
    (return (Math|Vector|MakeVector (.x (+ (Math|Vector2D|MakeVector2D (.x _returnvalue_3) (.y _returnvalue_3)) (* (Math|Vector2D|MakeVector2D (.x _worlddirection) (.y _worlddirection)) (/ (- (.z (Transformation|GetActorLocation (Utilities|Array|Get(acopy) _outactors))) (.z _returnvalue_3)) (.z _worlddirection))))) (.y (+ (Math|Vector2D|MakeVector2D (.x _returnvalue_3) (.y _returnvalue_3)) (* (Math|Vector2D|MakeVector2D (.x _worlddirection) (.y _worlddirection)) (/ (- (.z (Transformation|GetActorLocation (Utilities|Array|Get(acopy) _outactors))) (.z _returnvalue_3)) (.z _worlddirection))))) (.z (Transformation|GetActorLocation (Utilities|Array|Get(acopy) _outactors)))))))