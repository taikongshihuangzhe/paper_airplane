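; BP_enemy is an enemy actor that homes in on the player.
; On BeginPlay it disables collision and a timeline scales it up from zero to full size; collision is set off again when that finishes.
; Each Tick it moves toward the player at Speed with a swept offset and turns to face them.
; At zero HP or below it only sets a Dead flag, as the DestroyActor node is never executed.
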(event EventBeginPlay
  (Collision|SetActorEnableCollision false)
  (bind _alpha (Timeline|spawnTimeline Play)
    (:Update
      (Transformation|SetActorScale3D (Math|Conversions|ToVector(Float) (Math|Float|Lerp 0.0 1.0 _alpha))))
    (:Finished
      (Collision|SetActorEnableCollision false))))

(event EventTick
  (params (DeltaSeconds :type Float%20%28single-precision%29))
  (bind _hp (Variables|Default|GetHP))
  (bind _returnvalue (<= _hp 0.0))
  (CallFunction|MoveTowardsPlayer)
  (Variables|Default|SetDeltaSec DeltaSeconds)
  (if _returnvalue
    (Variables|Default|SetDead _returnvalue)))

(fn ConstructionScript)

(fn MoveTowardsPlayer
  (bind _player (Variables|Default|GetPlayer))
  (if true
    (Transformation|AddActorWorldOffset (* (Math|Vector|Normalize (- (Transformation|GetActorLocation _player) (Transformation|GetActorLocation))) (* (Utilities|Time|GetWorldDeltaSeconds) (Variables|Default|GetSpeed))) true)
    (Transformation|SetActorRotation (Math|Rotator|FindLookatRotation (Transformation|GetActorLocation) (Transformation|GetActorLocation _player)))))