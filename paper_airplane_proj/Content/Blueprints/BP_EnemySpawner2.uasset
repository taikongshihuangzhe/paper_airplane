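; Enemy spawner actor that creates BP_Enemy_Child while the plane_gameMode enemy count is below its maximum.
; BeginPlay caches the game mode and sets a named timer on SpawnEnemy, with no interval or looping specified.
; SpawnEnemy calls itself when kills are a multiple of five differing from CurrentEnemiesKilled, which is never updated here.
; It spawns after a random Delay whose range is zero, with no transform specified.
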(event Custom|SpawnEnemy
  (bind _bp_gamemode (Variables|Default|GetBP_GameMode))
  (bind _enemieskilled (Variables|/Game/Blueprints/plane_gameMode.plane_gameMode_C|GetEnemiesKilled _bp_gamemode))
  (if (< (Variables|/Game/Blueprints/plane_gameMode.plane_gameMode_C|GetEnemyCount _bp_gamemode) (Variables|/Game/Blueprints/plane_gameMode.plane_gameMode_C|GetMaxEnemies _bp_gamemode))
    (if (and (== (Math|Integer|%(Integer) _enemieskilled 5) 0) (!= _enemieskilled (Variables|Default|GetCurrentEnemiesKilled)))
      (CallFunction|SpawnEnemy))
    (Utilities|FlowControl|Delay (Math|Random|RandomFloatinRange 0.0 0.0))
    (Game|SpawnActorfromClass "/Game/Blueprints/BP_Enemy_Child.BP_Enemy_Child_C" (Math|Transform|MakeTransform "0, 0, 0" "0, 0, 0" "1,1,1") "Undefined" 0 0)))

(event EventBeginPlay
  (bind _asplane_game_mode (Utilities|Casting|CastToplane_gameMode (Game|GetGameMode)))
  (Variables|Default|SetBP_GameMode _asplane_game_mode)
  (Utilities|FlowControl|Sequence
    (:then_0
      (Utilities|Time|SetTimerbyFunctionName 0 "SpawnEnemy" 0.0))))

(event Collision|EventActorBeginOverlap
  (params (OtherActor :type Actor%20Object%20Reference)))

(event EventTick
  (params (DeltaSeconds :type Float%20%28single-precision%29)))

(fn ConstructionScript)