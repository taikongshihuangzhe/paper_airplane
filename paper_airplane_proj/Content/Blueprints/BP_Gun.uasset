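; Auto-firing gun actor that spawns type A or B projectiles from GunA on looping timers, starting with A at level 1 on BeginPlay.
; BulletControl routes type and level (1 or 2) to handlers that start or clear the timer, taking speed, damage and period from per-type info maps.
; PickUpBullet stops current fire and calls IfCurrentBulletType to choose the next type and level, but never updates the current ones.
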(event Custom|PickUpBullet
  (params (Type :type Integer))
  ;[1 1 1] PickUpBullet
  (CallFunction|BulletControl (Variables|Default|GetCurrentProjectileType) (Variables|Default|GetCurrentProjectileLevel) false)
  (bind (_outtype _outlevel) (CallFunction|IfCurrentBulletType Type))
  (CallFunction|BulletControl _outtype _outlevel true))

(event EventBeginPlay
  ;[1 1 1] Fire
  (bind _output_get (Variables|Default|SetCurrentProjectileType 0))
  (bind _output_get_2 (Variables|Default|SetCurrentProjectileLevel 1))
  (CallFunction|BulletControl _output_get _output_get_2 true))

(fn ConstructionScript)

(fn FireBulletAPrimary
  (Game|SpawnActorfromClass "/Game/Blueprints/Bullet/BP_BulletA.BP_BulletA_C" (Transformation|GetWorldTransform (Variables|Default|GetGunA)) "AlwaysSpawn" 0 "(R=0.926042,G=0.801905,B=0.147689,A=1.000000)" (Variables|Default|GetSpeed) (Variables|Default|GetDamage) self))

(fn FireBulletBPrimary
  (Game|SpawnActorfromClass "/Game/Blueprints/Bullet/BP_BulletB.BP_BulletB_C" (Transformation|GetWorldTransform (Variables|Default|GetGunA)) "AlwaysSpawn" 0 "(R=0.926042,G=0.801905,B=0.147689,A=0.000000)" (Variables|Default|GetSpeed) (Variables|Default|GetDamage) self))

(fn CalcDamageA
  (return (* (+ (Variables|Default|GetCurrentProjectileLevel) 1) 5.0)))

(fn CalcDamageB
  (return (* (+ (Variables|Default|GetCurrentProjectileLevel) 1) 1e+01)))

(fn StopBulletA
  (Utilities|Time|ClearTimerbyFunctionName 0 "FireBulletA_Primary"))

(fn IfCurrentBulletType
  (params (Type :type Integer))
  (switch int Type
    (:Default
      (return (LocalVariables|GetCalcLevel) (LocalVariables|GetCalcType)))
    (:0
      (if (== (Variables|Default|GetCurrentProjectileType) 0)
        (LocalVariables|SetCalcLevel (+ (Variables|Default|GetCurrentProjectileLevel) 1))
        (else
          (LocalVariables|SetCalcType 0)
          (LocalVariables|SetCalcLevel 0))))
    (:1
      (if (== (Variables|Default|GetCurrentProjectileType) 1)
        (LocalVariables|SetCalcLevel (+ (Variables|Default|GetCurrentProjectileLevel) 1))
        (else
          (LocalVariables|SetCalcType 1)
          (LocalVariables|SetCalcLevel 0))))))

(fn BulletControl
  (params (Type :type Integer) (Level :type Integer) (Set :type Boolean))
  (bind _bulletainfo (Variables|Default|GetBulletAInfo))
  (bind _bulletbinfo (Variables|Default|GetBulletBInfo))
  (bind _value (Utilities|Map|Find _bulletainfo Level))
  (bind _value_2 (Utilities|Map|Find _bulletbinfo Level))
  (switch int Type
    (:0
      (switch int Level
        (:1
          (CallFunction|BulletControlA0 Set _value))
        (:2
          (CallFunction|BulletControlA1 Set _value))))
    (:1
      (switch int Level
        (:1
          (CallFunction|BulletControlB0 Set _value_2))
        (:2
          (CallFunction|BulletControlB1 Set _value_2))))))

(fn BulletControlA0
  (params (Set :type Boolean) (BulletInfo :type Bullet%20Level%20Structure))
  (bind (_damage _spawn_period _speed) (Utilities|Struct|BreakBullet_Level BulletInfo))
  (if Set
    (Variables|Default|SetSpeed _speed)
    (Variables|Default|SetDamage _damage)
    (Utilities|Time|SetTimerbyFunctionName 0 "FireBulletA_Primary" _spawn_period true)
    (else
      (CallFunction|StopBulletA))))

(fn BulletControlA1
  (params (Set :type Boolean) (BulletInfo :type Bullet%20Level%20Structure))
  (bind (_damage _spawn_period _speed) (Utilities|Struct|BreakBullet_Level BulletInfo))
  (if Set
    (Utilities|Time|SetTimerbyFunctionName 0 "FireBulletA_Primary" _spawn_period true)
    (Variables|Default|SetDamage _damage)
    (Variables|Default|SetSpeed _speed)
    (CallFunction|FireBulletAPrimary)
    (else
      (CallFunction|StopBulletA))))

(fn StopBulletB
  (Utilities|Time|ClearTimerbyFunctionName 0 "FireBulletB_Primary"))

(fn BulletControlB0
  (params (Set :type Boolean) (BulletInfo :type Bullet%20Level%20Structure))
  (bind (_damage _spawn_period _speed) (Utilities|Struct|BreakBullet_Level BulletInfo))
  (if Set
    (Utilities|Time|SetTimerbyFunctionName 0 "FireBulletB_Primary" _spawn_period true)
    (Variables|Default|SetDamage _damage)
    (Variables|Default|SetSpeed _speed)
    (CallFunction|FireBulletBPrimary)
    (else
      (CallFunction|StopBulletB))))

(fn BulletControlB1
  (params (Set :type Boolean) (BulletInfo :type Bullet%20Level%20Structure))
  (bind (_damage _spawn_period _speed) (Utilities|Struct|BreakBullet_Level BulletInfo))
  (if Set
    (Utilities|Time|SetTimerbyFunctionName 0 "FireBulletB_Primary" _spawn_period true)
    (Variables|Default|SetDamage _damage)
    (Variables|Default|SetSpeed _speed)
    (CallFunction|FireBulletBPrimary)
    (else
      (CallFunction|StopBulletB))))