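; Base enemy Blueprint, apparently for a plane game, that registers itself with plane_gameMode's enemy count on BeginPlay and starts at MaxHealth.
; When movement is enabled, Tick selects by MoveType between swept straight-line movement and a curve movement that is still an empty stub.
; GotHit subtracts damage from Health when damage is enabled, then calls a death check whose result is not yet acted on.
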(event Custom|Got%20Hit
  (params (Damage :type Float%20%28single-precision%29))
  ;[1 0 0] Damage
  (if (Variables|Default|GetDamageEnabled)
    (CallFunction|CalculateDamage Damage)
    (CallFunction|GetIsDead)))

(event EventBeginPlay
  ;[1 1 1] Initianization
  (bind _asplane_game_mode (Utilities|Casting|CastToplane_gameMode (Game|GetGameMode)))
  (bind _output_get (Variables|Default|SetBP_GameMode _asplane_game_mode))
  (Default|UpdateEnemyCount _output_get 1)
  (Variables|Default|SetHealth (Variables|Default|GetMaxHealth)))

(event EventTick
  (params (DeltaSeconds :type Float%20%28single-precision%29))
  ;[0 0.2742 1] Movement
  (Variables|Default|Setdelta_t DeltaSeconds)
  (if (Variables|Default|GetMoveEnabled)
    (switch int (Variables|Default|GetMoveType)
      (:Default)
      (:0
        (CallFunction|SimpleMovement))
      (:1
        (CallFunction|CurveMovement)))))

(fn ConstructionScript)

(fn SimpleMovement
  (Transformation|SetActorLocation (+ (Transformation|GetActorLocation) (* (Variables|Default|GetSimpleMoveDirection) (* (Variables|Default|Getdelta_t) (Variables|Default|GetSimplyMoveSpeed)))) true false))

(fn CurveMovement)

(fn CalculateDamage
  (params (input_damage :type Float%20%28single-precision%29))
  (Variables|Default|SetHealth (- (Variables|Default|GetHealth) input_damage)))

(fn GetIsDead
  (return (<= (Variables|Default|GetHealth) 0.0)))