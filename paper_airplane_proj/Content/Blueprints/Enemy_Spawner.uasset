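; Enemy spawner actor that spawns enemies on a timeline defined by the Enemy_spawn_sheet data table.
; BeginPlay caches the table rows in an array and makes plane_gameState a tick prerequisite.
; Tick compares GameTime to the current row's Time, spawning at most one enemy per frame in row order and playing its move animation once.
; Only Time is read from each row; transform, health and damage are hardcoded.
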(event EventBeginPlay
  (bind _outrownames (DataTable|GetDataTableRowNames "/Game/Data/enemy_spawn_sheet.enemy_spawn_sheet"))
  (for _array_element _outrownames
    (bind _returnvalue (Utilities|GetDataTableRow "/Game/Data/enemy_spawn_sheet.enemy_spawn_sheet" _array_element)
      (:then
        (Utilities|Array|Add (Variables|Default|GetEnemy_spawn_array) _returnvalue))))
  (Variables|Default|SetEnemy_spawn_total (Utilities|Array|Length (Variables|Default|GetEnemy_spawn_array)))
  (bind _asplane_game_state (Utilities|Casting|CastToplane_gameState (Game|GetGameState)))
  (bind _output_get (Variables|Default|SetGame_state _asplane_game_state))
  (Actor|Tick|AddTickPrerequisiteActor _output_get))

(event EventTick
  (params (DeltaSeconds :type Float%20%28single-precision%29))
  (bind _game_state (Variables|Default|GetGame_state))
  (bind _gametime (Variables|/Game/Blueprints/plane_gameState.plane_gameState_C|GetgameTime _game_state))
  (if (<= (Variables|Default|GetEnemy_index) (Variables|Default|GetEnemy_spawn_total))
    (if (>= _gametime (Utilities|Struct|BreakEnemy_spawn_unit (Utilities|Array|Get(acopy) (Variables|Default|GetEnemy_spawn_array) (Variables|Default|GetEnemy_index))))
      (Development|PrintString (Utilities|String|ToString(Float) _gametime))
      (bind _returnvalue (Game|SpawnActorfromClass 0 (Math|Transform|MakeTransform "0, 0,120.000000" "0, 0, 0" "5.000000,5.000000,5.000000") "Undefined" 0 1e+01 5.0 0 0))
      (Components|Animation|PlayAnimation (Variables|Default|Gettransform_animmove1 _returnvalue) 0 false)
      (Math|Integer|IncrementInt (Variables|Default|GetEnemy_index)))))

(fn ConstructionScript)